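; BP_TurretHead is a hazard turret head that tracks and shoots at the player.
; A Tick state machine switches between Idle, Alert and Disabled, changing glow materials per state.
; Vision-cone overlaps plus a line trace trigger Alert, which rotates toward the player and spawns projectiles on a cooldown.
; Projectile hits disable it; an Inactive event for timed reactivation exists but is not called here.
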(event OnComponentBeginOverlap(VisionCone)
  (params (OverlappedComponent :type Primitive%20Component%20Object%20Reference) (OtherActor :type Actor%20Object%20Reference) (OtherComp :type Primitive%20Component%20Object%20Reference) (OtherBodyIndex :type Integer) (bFromSweep :type Boolean) (SweepResult :type Hit%20Result%20Structure%20%28by%20ref%29))
  ;[0.15 0.15 0.15 0.5] Collisions and Lines
  (if (Actor|ActorHasTag OtherActor "Player")
    (Variables|Default|SetPlayerInCone true)))

(event OnComponentEndOverlap(VisionCone)
  (params (OverlappedComponent :type Primitive%20Component%20Object%20Reference) (OtherActor :type Actor%20Object%20Reference) (OtherComp :type Primitive%20Component%20Object%20Reference) (OtherBodyIndex :type Integer))
  ;[0.15 0.15 0.15 0.5] Collisions and Lines
  (if (Actor|ActorHasTag OtherActor "Player")
    (Variables|Default|SetPlayerInCone false)))

(event Custom|Fire
  ;[0.15 0.15 0.15 0.5] Alert - Code active when the player is in the turret's cone of vision.
  (bind _returnvalue (Game|SpawnActorfromClass "/Game/COMP2150/Hazards/BP_Hazard_TurretProjectile.BP_Hazard_TurretProjectile_C" (Math|Transform|MakeTransform (Transformation|GetWorldLocation (Variables|Default|GetVision)) (Transformation|GetActorRotation)) "AlwaysSpawn" "MultiplyWithRoot" 0 0))
  (Variables|Default|SetCooldownTimer (Variables|Default|GetCooldownRate))
  (Collision|IgnoreActorwhenMoving (Variables|/Game/COMP2150/Hazards/BP_Hazard_TurretProjectile.BP_Hazard_TurretProjectile_C|GetMesh _returnvalue) self true))

(event Custom|Inactive
  ;[0.15 0.15 0.15 0.5] Inactive Code - Runs when Turret is in Inactive mode
  (Components|Activation|SetActive (Variables|Default|GetVisionCone) false false)
  (Utilities|FlowControl|Delay (Variables|Default|GetInactiveTime))
  (Components|Activation|SetActive (Variables|Default|GetVision) true false)
  (Variables|Default|SetState "NewEnumerator2")
  (Rendering|Material|SetMaterial (Variables|Default|GetHead) 1 "/Game/COMP2150/M_GlowYellow.M_GlowYellow"))

(event Custom|IdleMode
  ;[0.15 0.15 0.15 0.5] Idle - Code executed when the turret is active, but cannot see the player.
  (Transformation|SetActorRotation (Class|KismetMathLibrary|RInterptoConstant (Transformation|GetActorRotation) (Variables|Default|GetIdleView) (Utilities|Time|GetWorldDeltaSeconds) (Variables|Default|GetRotationSpeed))))

(event Custom|AlertMode
  ;[0.15 0.15 0.15 0.5] Alert - Code active when the player is in the turret's cone of vision.
  (CallFunction|LookatTarget)
  (CallFunction|CheckforLineOfSight)
  (bind _output_get (Variables|Default|SetCooldownTimer (- (Variables|Default|GetCooldownTimer) (Utilities|Time|GetWorldDeltaSeconds))))
  (if (< _output_get 0.0)
    (CallFunction|Fire)))

(event Custom|CheckForLineOfSight
  ;[0.15 0.15 0.15 0.5] Collisions and Lines
  (bind _outhit (Collision|LineTraceForObjects (Transformation|GetActorLocation) (Transformation|GetActorLocation (Game|Player|GetPlayerPawn 0)) (Variables|Default|GetObject%20Types) false 0 "None"))
  (if (Actor|ActorHasTag (.HitActor (Collision|BreakHitResult _outhit)) "Player")
    (Variables|Default|SetState "NewEnumerator3")
    (Rendering|Material|SetMaterial (Variables|Default|GetHead) 1 "/Game/COMP2150/M_GlowRed.M_GlowRed")
    (else
      (Variables|Default|SetState "NewEnumerator2")
      (Rendering|Material|SetMaterial (Variables|Default|GetHead) 1 "/Game/COMP2150/M_GlowYellow.M_GlowYellow"))))

(event Custom|LookAtTarget
  ;[0.15 0.15 0.15 0.5] Alert - Code active when the player is in the turret's cone of vision.
  (Transformation|SetActorRotation (Class|KismetMathLibrary|RInterptoConstant (Transformation|GetActorRotation) (Math|Rotator|FindLookatRotation (Transformation|GetActorLocation) (Transformation|GetWorldLocation (Variables|/Script/Engine.Character|GetCapsuleComponent (Game|GetPlayerCharacter 0)))) (Utilities|Time|GetWorldDeltaSeconds) (Variables|Default|GetRotationSpeed))))

(event EventBeginPlay
  ;[0.15 0.15 0.15 0.5] Start and Tick
  (Variables|Default|SetState "NewEnumerator2")
  (Variables|Default|SetIdleView (Transformation|GetActorRotation)))

(event Collision|EventHit
  (params (MyComp :type Primitive%20Component%20Object%20Reference) (Other :type Actor%20Object%20Reference) (OtherComp :type Primitive%20Component%20Object%20Reference) (bSelfMoved :type Boolean) (HitLocation :type Vector :default "0, 0, 0") (HitNormal :type Vector :default "0, 0, 0") (NormalImpulse :type Vector :default "0, 0, 0") (Hit :type Hit%20Result%20Structure%20%28by%20ref%29))
  ;[0.15 0.15 0.15 0.5] Collisions and Lines
  (if (Actor|ActorHasTag Other "Projectile")
    (Variables|Default|SetState "NewEnumerator1")))

(event EventTick
  (params (DeltaSeconds :type Float%20%28single-precision%29))
  ;[0.15 0.15 0.15 0.5] Start and Tick
  (switch Utilities|FlowControl|Switch|SwitchonETurretStates (Variables|Default|GetState)
    (:NewEnumerator1
      (Rendering|Material|SetMaterial (Variables|Default|GetHead) 0 "/Game/COMP2150/M_GlowBlue.M_GlowBlue"))
    (:NewEnumerator2
      (CallFunction|IdleMode)
      (if (Variables|Default|GetPlayerInCone)
        (CallFunction|CheckforLineOfSight)))
    (:NewEnumerator3
      (CallFunction|AlertMode)
      (if (not (Variables|Default|GetPlayerInCone))
        (Variables|Default|SetState "NewEnumerator2")
        (Rendering|Material|SetMaterial (Variables|Default|GetHead) 1 "/Game/COMP2150/M_GlowYellow.M_GlowYellow")))))

(fn ConstructionScript)