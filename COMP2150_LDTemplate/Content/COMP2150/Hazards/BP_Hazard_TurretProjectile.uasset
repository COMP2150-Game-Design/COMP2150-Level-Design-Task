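; BP_Hazard_TurretProjectile is a turret projectile hazard that launches itself along its forward vector with a mesh impulse on spawn.
; On hitting a component tagged Shield, it receives a half-strength impulse along the hit normal to deflect it and calls ShieldHit on BP_Sinead, printing a message if that cast fails.
; Any other hit destroys the projectile after a one-tick delay.
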(event EventBeginPlay
  (Physics|AddImpulse (Variables|Default|GetMesh) (* (Transformation|GetActorForwardVector) (Variables|Default|GetLaunchForce)) "None" false))

(event Collision|EventHit
  (params (MyComp :type Primitive%20Component%20Object%20Reference) (Other :type Actor%20Object%20Reference) (OtherComp :type Primitive%20Component%20Object%20Reference) (bSelfMoved :type Boolean) (HitLocation :type Vector :default "0, 0, 0") (HitNormal :type Vector :default "0, 0, 0") (NormalImpulse :type Vector :default "0, 0, 0") (Hit :type Hit%20Result%20Structure%20%28by%20ref%29))
  (if (Components|ComponentHasTag OtherComp "Shield")
    (Physics|AddImpulse (Variables|Default|GetMesh) (* HitNormal (/ (Variables|Default|GetLaunchForce) 2.0)) "None" false)
    (bind _asbp_sinead (Utilities|Casting|CastToBP_Sinead Other)
      (:then
        (Default|ShieldHit _asbp_sinead))
      (:CastFailed
        (Development|PrintString "\"No BP_Sinead attached to shield\"")))
    (else
      (Utilities|FlowControl|DelayUntilNextTick)
      (Actor|DestroyActor))))

(fn ConstructionScript
  (|CallParentFunction))