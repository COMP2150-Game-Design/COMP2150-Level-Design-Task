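; BP_EndGameDoor is an end-of-level door that opens once the player has collected three keys and leads to another level.
; Tick mirrors the key count from BP_2150GameMode, and a player-tagged overlap on TriggerBox sets Open when that count is three.
; While open, Tick lerps the door's relative location toward TargetLocation, scaled by DoorSpeed and delta time.
; Any overlap on the Exit volume opens LevelToLoad, with no tag or door-state check.
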(event OnComponentBeginOverlap(TriggerBox)
  (params (OverlappedComponent :type Primitive%20Component%20Object%20Reference) (OtherActor :type Actor%20Object%20Reference) (OtherComp :type Primitive%20Component%20Object%20Reference) (OtherBodyIndex :type Integer) (bFromSweep :type Boolean) (SweepResult :type Hit%20Result%20Structure%20%28by%20ref%29))
  (if (Actor|ActorHasTag OtherActor "Player")
    (if (== (Variables|Default|GetKeys) 3)
      (Variables|Default|SetOpen true)
      (Development|PrintString "Lets open!"))))

(event OnComponentBeginOverlap(Exit)
  (params (OverlappedComponent :type Primitive%20Component%20Object%20Reference) (OtherActor :type Actor%20Object%20Reference) (OtherComp :type Primitive%20Component%20Object%20Reference) (OtherBodyIndex :type Integer) (bFromSweep :type Boolean) (SweepResult :type Hit%20Result%20Structure%20%28by%20ref%29))
  (Development|PrintString "Exit overlapped")
  (Game|OpenLevel(byObjectReference) (Utilities|Struct|BreakSoftWorldReference (Variables|Default|GetLevelToLoad))))

(event Custom|MoveDoor
  (bind _door (Variables|Default|GetDoor))
  (Transformation|SetRelativeLocation _door (Math|Vector|Lerp(Vector) (.Location (Math|Transform|BreakTransform (Transformation|GetRelativeTransform _door))) (Variables|Default|GetTargetLocation) (* (Variables|Default|GetDoorSpeed) (Utilities|Time|GetWorldDeltaSeconds))) false false))

(event EventBeginPlay
  (bind _asbp_2150game_mode (Utilities|Casting|CastToBP_2150GameMode (Game|GetGameMode)))
  (Variables|Default|SetGameMode _asbp_2150game_mode))

(event EventTick
  (params (DeltaSeconds :type Float%20%28single-precision%29))
  (Variables|Default|SetKeys (Variables|/Game/COMP2150/Core/MainGame/BP_2150GameMode.BP_2150GameMode_C|GetKeys (Variables|Default|GetGameMode)))
  (if (Variables|Default|GetOpen)
    (CallFunction|MoveDoor)))

(fn ConstructionScript)