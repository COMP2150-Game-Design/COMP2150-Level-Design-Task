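; Gun turret hazard that turns to track the player and fires projectiles, using a two-state Idle/Alert machine run on Tick.
; Vision cone overlap with a Player-tagged actor triggers Alert if a WorldStatic line trace is clear, checked only on entry; leaving returns to Idle.
; Alert enlarges the vision and spawns self-ignoring projectiles from the barrel on a cooldown.
; Idle restores the vision size and eases rotation back to the starting view.
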(event OnComponentBeginOverlap(VisionCone)
  (params (OverlappedComponent :type Primitive%20Component%20Object%20Reference) (OtherActor :type Actor%20Object%20Reference) (OtherComp :type Primitive%20Component%20Object%20Reference) (OtherBodyIndex :type Integer) (bFromSweep :type Boolean) (SweepResult :type Hit%20Result%20Structure%20%28by%20ref%29))
  (if (Actor|ActorHasTag OtherActor "Player")
    (bind _returnvalue (Collision|LineTraceForObjects (Transformation|GetWorldLocation (Variables|Default|GetVisionCone)) (Transformation|GetActorLocation OtherActor) (Utilities|Array|MakeArray "ObjectTypeQuery1") false 0 "None"))
    (if (not _returnvalue)
      (if (Utilities|Enum|Equal(Enum) (Variables|Default|GetState) "NewEnumerator2")
        (Variables|Default|SetState "NewEnumerator3")
        (CallFunction|AlertModeInit)
        (Development|PrintString "Switching to Alert")))))

(event OnComponentEndOverlap(VisionCone)
  (params (OverlappedComponent :type Primitive%20Component%20Object%20Reference) (OtherActor :type Actor%20Object%20Reference) (OtherComp :type Primitive%20Component%20Object%20Reference) (OtherBodyIndex :type Integer))
  (if (Actor|ActorHasTag OtherActor "Player")
    (if (Utilities|Enum|Equal(Enum) (Variables|Default|GetState) "NewEnumerator3")
      (Variables|Default|SetState "NewEnumerator2")
      (CallFunction|IdleModeInit))))

(event Custom|Fire
  ;[0.15 0.15 0.15 0.5] Alert - Code active when the player is in the turret's cone of vision.
  (bind _returnvalue (Game|SpawnActorfromClass "/Game/COMP2150/Hazards/BP_Hazard_TurretProjectile.BP_Hazard_TurretProjectile_C" (Math|Transform|MakeTransform (Transformation|GetWorldLocation (Variables|Default|GetBarrel/Eyes)) (Transformation|GetActorRotation)) "AlwaysSpawn" "MultiplyWithRoot" 0 0))
  (Variables|Default|SetCooldownTimer (Variables|Default|GetCooldown))
  (Collision|IgnoreActorwhenMoving (Variables|/Game/COMP2150/Hazards/BP_Hazard_TurretProjectile.BP_Hazard_TurretProjectile_C|GetStaticMesh _returnvalue) self true))

(event Custom|LookAtTarget
  (bind _output_get (Variables|Default|SetTargetLocation (Transformation|GetActorLocation (Game|GetPlayerCharacter 0))))
  (Transformation|SetActorRotation (Math|Rotator|Lerp(Rotator) (Transformation|GetActorRotation) (Math|Rotator|FindLookatRotation (Transformation|GetActorLocation) _output_get) (* (Utilities|Time|GetWorldDeltaSeconds) (Variables|Default|GetRotationSpeed)) true)))

(event Custom|AlertModeInit
  (bind _vision (Variables|Default|GetVision))
  ;[0.15 0.15 0.15 0.5] Alert - Code active when the player is in the turret's cone of vision.
  (Transformation|SetWorldScale3D _vision (+ (Transformation|GetWorldScale _vision) (Variables|Default|GetAlertConeGrowth))))

(event Custom|IdleMode
  ;[0.15 0.15 0.15 0.5] Idle - Code executed when the turret is active, but cannot see the player.
  (Transformation|SetActorRotation (Math|Rotator|Lerp(Rotator) (Transformation|GetActorRotation) (Variables|Default|GetIdleView) (* (Utilities|Time|GetWorldDeltaSeconds) (Variables|Default|GetRotationSpeed)) true)))

(event Custom|AlertMode
  ;[0.15 0.15 0.15 0.5] Alert - Code active when the player is in the turret's cone of vision.
  (CallFunction|LookatTarget)
  (if (> (Variables|Default|GetCooldownTimer) 0.0)
    (Variables|Default|SetCooldownTimer (- (Variables|Default|GetCooldownTimer) (Utilities|Time|GetWorldDeltaSeconds)))
    (else
      (CallFunction|Fire))))

(event Custom|IdleModeInit
  (bind _vision (Variables|Default|GetVision))
  ;[0.15 0.15 0.15 0.5] Idle - Code executed when the turret is active, but cannot see the player.
  (Transformation|SetWorldScale3D _vision (- (Transformation|GetWorldScale _vision) (Variables|Default|GetAlertConeGrowth))))

(event EventBeginPlay
  (Variables|Default|SetState "NewEnumerator2")
  (Variables|Default|SetIdleView (Transformation|GetActorRotation)))

(event EventTick
  (params (DeltaSeconds :type Float%20%28single-precision%29))
  (switch Utilities|FlowControl|Switch|SwitchonETurretStates (Variables|Default|GetState)
    (:NewEnumerator2
      (CallFunction|IdleMode))
    (:NewEnumerator3
      (CallFunction|AlertMode))))

(event Custom|DebugCone
  (params (Duration :type Float%20%28single-precision%29))
  (Class|KismetSystemLibrary|DrawDebugConeinDegrees (Transformation|GetActorLocation) (Math|Rotator|GetRotationXVector (Transformation|GetActorRotation)) 1e+02 45.0 45.0 12 "(R=0.427083,G=0.065519,B=0.000000,A=1.000000)" Duration 1.0 "Foreground"))

(fn ConstructionScript)