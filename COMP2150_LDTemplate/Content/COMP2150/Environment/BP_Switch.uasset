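; BP_Switch is a clickable environment switch that triggers another actor, its Receiver.
; ClickTriggered finds the BP_SwitchReceiver component on the Receiver and calls Triggered on it.
; SetHighlight stores a flag, which Tick reads every frame to tint the Sphere's materials orange or black.
; The construction script draws a temporary debug line from the switch's location, with no end point set.
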(event Custom|ClickTriggered
  (Default|Triggered (Actor|GetComponentbyClass (Variables|Default|GetReceiver) "/Game/COMP2150/Environment/BP_SwitchReceiver.BP_SwitchReceiver_C")))

(event Custom|SetHighlight
  (params (Input :type Boolean))
  (Variables|Default|SetHighlighted Input))

(event EventBeginPlay)

(event Collision|EventActorBeginOverlap
  (params (OtherActor :type Actor%20Object%20Reference)))

(event EventTick
  (params (DeltaSeconds :type Float%20%28single-precision%29))
  (bind _sphere (Variables|Default|GetSphere))
  (if (Variables|Default|GetHighlighted)
    (Rendering|Material|SetColorParameterValueonMaterials _sphere "Color" "(R=1.000000,G=0.379659,B=0.000000,A=1.000000)")
    (else
      (Rendering|Material|SetColorParameterValueonMaterials _sphere "Color" "(R=0.000000,G=0.000000,B=0.000000,A=1.000000)"))))

(fn ConstructionScript
  (Rendering|Debug|DrawDebugLine :LineStart (Transformation|GetActorLocation) :Duration 1e+01 :Thickness 2e+01 :DepthPriority "Foreground"))